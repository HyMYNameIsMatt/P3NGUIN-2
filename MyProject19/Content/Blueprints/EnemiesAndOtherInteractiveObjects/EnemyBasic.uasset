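; Basic enemy that the player can grab, carry toward the cursor direction, drop, throw or launch away from themselves.
; Tick pins a grabbed enemy to the player or moves a launched one manually, pausing while the TimeDecider game instance has time stopped.
; A short forward trace ricochets it off surfaces by mirroring yaw around the hit normal, with camera shake.
; Launch speed holds for a frictionless period, then decays per tick until it stops.
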(event Custom|Grab%20Enemy
  (if (Variables|Default|GetGrabbed)
    (Variables|Default|SetGrabbed false)
    (CallFunction|ThrowEnemy)
    (else
      (Variables|Default|SetGrabbed true)
      (Variables|Default|SetLaunched false))))

(event Custom|Throw%20Enemy
  (if (not (Variables|Default|GetGrabbed))
    (Variables|Default|SetLaunched true)
    (Variables|Default|SetLaunch%20Angle (Math|Rotator|FindLookatRotation (Transformation|GetActorLocation (Game|Player|GetPlayerPawn 0)) (Transformation|GetActorLocation)))
    (Variables|Default|SetLaunch%20Speed 2e+01)
    (Variables|Default|SetLaunch%20Frictionless%20Time (Variables|Default|GetLaunch%20Frictionless%20Time%20Edit))))

(event Custom|Launch%20Enemy
  (Variables|Default|SetLaunched true)
  (Variables|Default|SetLaunch%20Angle (Math|Rotator|FindLookatRotation (Transformation|GetActorLocation (Game|Player|GetPlayerPawn 0)) (Transformation|GetActorLocation)))
  (Variables|Default|SetLaunch%20Speed 4e+01)
  (Variables|Default|SetLaunch%20Frictionless%20Time (Variables|Default|GetLaunch%20Frictionless%20Time%20Edit)))

(event Custom|Let%20Go%20of%20Enemy
  (Variables|Default|SetGrabbed false))

(event EventBeginPlay
  (bind _asthird_person_character_2d (Utilities|Casting|CastToThirdPersonCharacter2D (Game|Player|GetPlayerPawn 0)))
  (bind _astime_decider (Utilities|Casting|CastToTimeDecider (Game|GetGameInstance))))

(event EventTick
  (params (DeltaSeconds :type Float%20%28single-precision%29))
  (bind _returnvalue (Transformation|GetActorLocation))
  (if (Variables|Default|GetGrabbed)
    (Transformation|SetActorLocation (+ (Transformation|GetActorLocation (Game|Player|GetPlayerPawn 0)) (Math|Vector|RotateVector "100.000000, 0, 0" (Variables|/Game/Blueprints/2D/Blueprints/Tests/ThirdPersonCharacter2D.ThirdPersonCharacter2D_C|GetCursorRotation (stale EventBeginPlay _asthird_person_character_2d)))) false false)
    (else
      (Utilities|FlowControl|Sequence
        (:then_0
          (if (Variables|Default|GetLaunched)
            (if (> (Variables|Default|GetLaunch%20Speed) 0.0)
              (if (not (Variables|/Game/Blueprints/TimeDecider.TimeDecider_C|GetTimeStopped (stale EventBeginPlay _astime_decider)))
                (bind (_outhit _returnvalue_2) (Collision|LineTraceByChannel _returnvalue (+ _returnvalue (Math|Vector|RotateVector (Math|Vector|MakeVector 75.0 0.0 0.0) (Variables|Default|GetLaunch%20Angle))) "TraceTypeQuery1" false 0 "None"))
                (if _returnvalue_2
                  (Class|PlayerController|ClientPlayCameraShake (Game|GetPlayerController 0) "/Game/Blueprints/CameraShakeCustom.CameraShakeCustom_C" 5.0 "World" "0, 0, 0")
                  (Variables|Default|SetLaunch%20Angle (Math|Rotator|MakeRotator 0.0 0.0 (- (+ (* (- (.Yaw (Math|Rotator|BreakRotator (Math|Rotator|FindLookatRotation (.ImpactPoint (Collision|BreakHitResult _outhit)) (+ (.ImpactPoint (Collision|BreakHitResult _outhit)) (* (.ImpactNormal (Collision|BreakHitResult _outhit)) 5e+03))))) (.Yaw (Math|Rotator|BreakRotator (Variables|Default|GetLaunch%20Angle)))) 2.0) (.Yaw (Math|Rotator|BreakRotator (Variables|Default|GetLaunch%20Angle)))) 1.8e+02))))
                (Transformation|SetActorLocation (+ (Transformation|GetActorLocation) (Math|Vector|RotateVector (Math|Vector|MakeVector (Variables|Default|GetLaunch%20Speed) 0.0 0.0) (Variables|Default|GetLaunch%20Angle))) true false)
                (if (<= (Variables|Default|GetLaunch%20Frictionless%20Time) 0.0)
                  (Variables|Default|SetLaunch%20Speed (- (Variables|Default|GetLaunch%20Speed) 0.2))))
              (else
                (Variables|Default|SetLaunched false)))))
        (:then_1
          (CallFunction|NoFrictionTimer))))))

(fn ConstructionScript)

(fn SendHealthtoBar1
  (params (Enemy%20Health :type Float%20%28single-precision%29))
  (bind _output_get (Variables|/Game/Blueprints/UI/EnemyHealth.EnemyHealth_C|SetHealthPercentageEnemy (Variables|Default|GetEnemyHealth) (/ Enemy%20Health (Variables|Default|GetMaxHealth1))))
  (Development|PrintString (Utilities|String|ToString(Float) _output_get)))

(fn SetHealthBarLocation)

(fn NoFrictionTimer
  (if (not (<= (Variables|Default|GetLaunch%20Frictionless%20Time) 0.0))
    (Variables|Default|SetLaunch%20Frictionless%20Time (- (Variables|Default|GetLaunch%20Frictionless%20Time) (* (Utilities|Time|GetWorldDeltaSeconds) (Math|Float|MakeLiteralFloat 1.0))))))