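; An object the player can grab and throw: GrabMe toggles holding it in front of the player, and releasing launches it away from them.
; Tick moves it manually rather than by physics, pausing flight while the TimeDecider game instance has time stopped.
; A short forward trace reflects the yaw off surfaces with a camera shake.
; Speed stays constant until the no-friction timer expires, then drops each tick until it stops.
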(event Custom|StartMeUp
  (if (not (Variables|Default|GetHeld))
    (Variables|Default|SetLaunched true)
    (Variables|Default|SetLaunch%20Angle (Math|Rotator|FindLookatRotation (Transformation|GetActorLocation (Game|Player|GetPlayerPawn 0)) (Transformation|GetActorLocation)))
    (Variables|Default|SetLaunch%20Speed 2e+01)
    (Variables|Default|SetLaunchNoFrictionTime (Variables|Default|GetLaunchNoFrictionTimeEDIT))))

(event Custom|Grab%20Me
  (if (Variables|Default|GetHeld)
    (Variables|Default|SetHeld false)
    (CallFunction|StartMeUp)
    (else
      (Variables|Default|SetHeld true)
      (Variables|Default|SetLaunched false))))

(event Collision|EventHit
  (params (MyComp :type Primitive%20Component%20Object%20Reference) (Other :type Actor%20Object%20Reference) (OtherComp :type Primitive%20Component%20Object%20Reference) (bSelfMoved :type Boolean) (HitLocation :type Vector :default "0, 0, 0") (HitNormal :type Vector :default "0, 0, 0") (NormalImpulse :type Vector :default "0, 0, 0") (Hit :type Hit%20Result%20Structure%20%28by%20ref%29))
  (Development|PrintString "the"))

(event Collision|EventActorBeginOverlap
  (params (OtherActor :type Actor%20Object%20Reference))
  (if (Utilities|ClassIsChildOf (Utilities|GetClass OtherActor) "/Script/Engine.BlockingVolume")
    _))

(event EventTick
  (params (DeltaSeconds :type Float%20%28single-precision%29))
  (bind _returnvalue (Transformation|GetActorLocation))
  (bind _returnvalue_2 (Game|Player|GetPlayerPawn 0))
  (if (Variables|Default|GetHeld)
    (Transformation|SetActorLocation (+ (Transformation|GetActorLocation _returnvalue_2) (Math|Vector|RotateVector "100.000000, 0, 0" (Transformation|GetActorRotation _returnvalue_2))) false false)
    (else
      (Utilities|FlowControl|Sequence
        (:then_0
          (if (Variables|Default|GetLaunched)
            (if (> (Variables|Default|GetLaunch%20Speed) 0.0)
              (bind _astime_decider (Utilities|Casting|CastToTimeDecider (Game|GetGameInstance)))
              (if (not (Variables|/Game/Blueprints/TimeDecider.TimeDecider_C|GetTimeStopped _astime_decider))
                (bind (_outhit _returnvalue_3) (Collision|LineTraceByChannel _returnvalue (+ _returnvalue (Math|Vector|RotateVector (Math|Vector|MakeVector 5e+01 0.0 0.0) (Variables|Default|GetLaunch%20Angle))) "TraceTypeQuery1" false 0 "None"))
                (if _returnvalue_3
                  (Development|PrintString (Utilities|String|ToString(Float) (.Yaw (Math|Rotator|BreakRotator (Math|Rotator|FindLookatRotation (.ImpactPoint (Collision|BreakHitResult _outhit)) (+ (.ImpactPoint (Collision|BreakHitResult _outhit)) (* (.ImpactNormal (Collision|BreakHitResult _outhit)) 5e+03)))))))
                  (Class|PlayerController|ClientPlayCameraShake (Game|GetPlayerController 0) "/Game/Blueprints/CameraShakeCustom.CameraShakeCustom_C" 5.0 "World" "0, 0, 0")
                  (Variables|Default|SetLaunch%20Angle (Math|Rotator|MakeRotator 0.0 0.0 (- (+ (* (- (.Yaw (Math|Rotator|BreakRotator (Math|Rotator|FindLookatRotation (.ImpactPoint (Collision|BreakHitResult _outhit)) (+ (.ImpactPoint (Collision|BreakHitResult _outhit)) (* (.ImpactNormal (Collision|BreakHitResult _outhit)) 5e+03))))) (.Yaw (Math|Rotator|BreakRotator (Variables|Default|GetLaunch%20Angle)))) 2.0) (.Yaw (Math|Rotator|BreakRotator (Variables|Default|GetLaunch%20Angle)))) 1.8e+02))))
                (Transformation|SetActorLocation (+ (Transformation|GetActorLocation) (Math|Vector|RotateVector (Math|Vector|MakeVector (Variables|Default|GetLaunch%20Speed) 0.0 0.0) (Variables|Default|GetLaunch%20Angle))) true false)
                (if (<= (Variables|Default|GetLaunchNoFrictionTime) 0.0)
                  (Variables|Default|SetLaunch%20Speed (- (Variables|Default|GetLaunch%20Speed) 0.2))))
              (else
                (Variables|Default|SetLaunched false)
                (Development|PrintString "Hello")))))
        (:then_1
          (CallFunction|NoFrictionTimer))))))

(fn ConstructionScript
  (|CallParentFunction))

(fn NoFrictionTimer
  (if (not (<= (Variables|Default|GetLaunchNoFrictionTime) 0.0))
    (Variables|Default|SetLaunchNoFrictionTime (- (Variables|Default|GetLaunchNoFrictionTime) (* (Utilities|Time|GetWorldDeltaSeconds) (Math|Float|MakeLiteralFloat 1.0))))))