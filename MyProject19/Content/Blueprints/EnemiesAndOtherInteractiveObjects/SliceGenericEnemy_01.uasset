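; Generic enemy character with a three-way spread shot, a poison shot, launch-based dodges and a forward lunge.
; Damage lowers health, updates its health-bar widget and notifies the player character; BeginPlay sets up health and activates it after a random delay.
; An action picker using time stop, screen visibility, player distance and random rolls, plus the death check, is disconnected; Tick is empty, so neither runs.
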(event Custom|Spread%20Shot
  (bind _returnvalue (Transformation|GetActorRotation))
  (bind _returnvalue_2 (Transformation|GetActorRotation))
  (bind _self self)
  (bind (_roll _pitch _yaw) (Math|Rotator|BreakRotator _returnvalue))
  (bind (_roll_2 _pitch_2 _yaw_2) (Math|Rotator|BreakRotator _returnvalue_2))
  ;[1 1 1] SpreadShot
  (Game|SpawnActorfromClass "/Game/Blueprints/EnemiesAndOtherInteractiveObjects/IAMBULLETHELLO.IAMBULLETHELLO_C" (Math|Transform|MakeTransform (Transformation|GetActorLocation) (Transformation|GetActorRotation)) "Undefined" 0 _self)
  (Game|SpawnActorfromClass "/Game/Blueprints/EnemiesAndOtherInteractiveObjects/IAMBULLETHELLO.IAMBULLETHELLO_C" (Math|Transform|MakeTransform (Transformation|GetActorLocation) (Math|Rotator|MakeRotator _roll_2 _pitch_2 (+ _yaw_2 3e+01))) "Undefined" 0 _self)
  (Game|SpawnActorfromClass "/Game/Blueprints/EnemiesAndOtherInteractiveObjects/IAMBULLETHELLO.IAMBULLETHELLO_C" (Math|Transform|MakeTransform (Transformation|GetActorLocation) (Math|Rotator|MakeRotator _roll _pitch (+ _yaw -3e+01))) "Undefined" 0 _self)
  (Variables|Default|SetBusyRightNow true))

(event Custom|PoisonShot
  ;[1 1 1] Poison Shot
  (Game|SpawnActorfromClass "/Game/Blueprints/EnemiesAndOtherInteractiveObjects/Poison.Poison_C" (Math|Transform|MakeTransform (Transformation|GetActorLocation) (Transformation|GetActorRotation)) "Undefined" 0 self)
  (Variables|Default|SetBusyRightNow true))

(event Custom|Dodge
  (bind _returnvalue (Transformation|GetActorRotation))
  (bind _returnvalue_2 (Math|Vector|GetRightVector _returnvalue))
  ;[1 1 1] Dodgetoleftorright
  (if (Math|Random|RandomBool)
    (Character|LaunchCharacter (* _returnvalue_2 2500) false false)
    (else
      (Character|LaunchCharacter (* _returnvalue_2 -2500) false false))))

(event Custom|MoveForward
  ;[1 1 1] DodgeForward
  (Character|LaunchCharacter (* (Math|Vector|GetForwardVector (Transformation|GetActorRotation)) 5000) false false)
  (Variables|Default|SetBusyRightNow true))

(event Custom|Dodge%20Back
  ;[1 1 1] MoveBack
  (Character|LaunchCharacter (* (Math|Vector|GetForwardVector (Transformation|GetActorRotation)) -2500) false false)
  (Variables|Default|SetBusyRightNow true))

(event Game|Damage|EventAnyDamage
  (params (Damage :type Float%20%28single-precision%29) (DamageType :type Damage%20Type%20Object%20Reference) (InstigatedBy :type Controller%20Object%20Reference) (DamageCauser :type Actor%20Object%20Reference))
  ;[1 1 1] TakeDamage
  (bind _output_get (Variables|Default|SetHealth_0 (- (Variables|Default|GetHealth_0) Damage)))
  (CallFunction|SendHealthtoBar0 _output_get)
  (Development|PrintString (Utilities|String|ToString(Float) _output_get) true true "(R=1.000000,G=0.061744,B=0.000000,A=1.000000)")
  (bind _asthird_person_character_2d (Utilities|Casting|CastToThirdPersonCharacter2D (Game|Player|GetPlayerPawn 0)))
  (Default|DamagedAnEnemyBonus _asthird_person_character_2d))

(event EventBeginPlay
  (bind _asenemy_health (Utilities|Casting|CastToEnemyHealth (UserInterface|GetUserWidgetObject (Variables|Default|GetMyHealth))))
  (Variables|Default|SetMyHpBar _asenemy_health)
  (bind _output_get (Variables|Default|SetHealth_0 25.0))
  (Variables|Default|SetMaxHealth_0 _output_get)
  (Utilities|FlowControl|Delay (Math|Random|RandomFloatinRange 0.0 3.0))
  (Variables|Default|SetActivated true))

(event EventTick
  (params (DeltaSeconds :type Float%20%28single-precision%29)))

(fn ConstructionScript
  (|CallParentFunction))

(fn SendHealthtoBar0
  (params (NewParam :type Float%20%28single-precision%29))
  (bind _output_get (Variables|/Game/Blueprints/UI/EnemyHealth.EnemyHealth_C|SetHealthPercentageEnemy (Variables|Default|GetMyHpBar) (/ NewParam (Variables|Default|GetMaxHealth_0))))
  (Development|PrintString (Utilities|String|ToString(Float) _output_get)))