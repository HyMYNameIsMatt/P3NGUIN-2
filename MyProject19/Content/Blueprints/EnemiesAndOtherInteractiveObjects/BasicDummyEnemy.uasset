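; BasicDummyEnemy is an enemy that faces the player and repeatedly spawns IAMBULLETHELLO projectiles.
; Tick gates firing with a BusyRightNow flag and two-second Delay, and only stops controller movement while the game instance's TimeDecider reports stopped time.
; AnyDamage lowers Health and updates the EnemyHealth widget.
; Tick separately checks Health1, spawning particles and removing widget and actor at zero or below.
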(event Game|Damage|EventAnyDamage
  (params (Damage :type Float%20%28single-precision%29) (DamageType :type Damage%20Type%20Object%20Reference) (InstigatedBy :type Controller%20Object%20Reference) (DamageCauser :type Actor%20Object%20Reference))
  (bind _output_get (Variables|Default|SetHealth (- (Variables|Default|GetHealth) Damage)))
  (CallFunction|SendHealthtoBar1 _output_get)
  (Development|PrintString (Utilities|String|ToString(Float) _output_get) true true "(R=1.000000,G=0.061744,B=0.000000,A=1.000000)"))

(event EventBeginPlay
  (bind _asenemy_health (Utilities|Casting|CastToEnemyHealth (UserInterface|GetUserWidgetObject (Variables|Default|GetHP))))
  (Variables|Default|SetEnemyHealth _asenemy_health)
  (Variables|Default|SetStartingLocation (Transformation|GetActorLocation))
  (CallFunction|SendHealthtoBar1 (Variables|Default|GetHealth))
  (if (not (Rendering|IsVisible (Variables|Character|GetMesh)))
    (Development|PrintString "I'm away")))

(event EventTick
  (params (DeltaSeconds :type Float%20%28single-precision%29))
  (Transformation|SetRelativeLocation (Variables|Default|GetHP) (Transformation|GetActorLocation) false false)
  (Utilities|FlowControl|Sequence
    (:then_0
      (bind _astime_decider (Utilities|Casting|CastToTimeDecider (Game|GetGameInstance)))
      (if (Variables|/Game/Blueprints/TimeDecider.TimeDecider_C|GetTimeStopped _astime_decider)
        (AI|Navigation|StopMovement (Pawn|GetController))
        (else
          (Utilities|FlowControl|Sequence
            (:then_0
              (Transformation|SetActorRelativeRotation (Math|Rotator|FindLookatRotation (Transformation|GetActorLocation self) (Transformation|GetActorLocation (Game|Player|GetPlayerPawn 0)))))
            (:then_1
              (if (Variables|Default|GetBusyRightNow)
                (Utilities|FlowControl|Delay 2.0)
                (Variables|Default|SetBusyRightNow false)
                (else
                  (Game|SpawnActorfromClass "/Game/Blueprints/EnemiesAndOtherInteractiveObjects/IAMBULLETHELLO.IAMBULLETHELLO_C" (Math|Transform|MakeTransform (Transformation|GetActorLocation) (Transformation|GetActorRotation)) "Undefined" 0 self)
                  (Variables|Default|SetBusyRightNow true))))))))
    (:then_1
      (if (<= (Variables|Default|GetHealth1) 0.0)
        (Effects|SpawnEmitteratLocation "/Game/Defaultpparticle.Defaultpparticle" (Transformation|GetActorLocation))
        (Widget|RemovefromParent (Variables|Default|GetEnemyHealth))
        (Actor|DestroyActor)))))

(fn ConstructionScript
  (|CallParentFunction))