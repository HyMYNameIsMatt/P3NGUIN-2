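; Proof-of-concept projectile actor that flies straight along its facing and freezes in place while time is stopped.
; BeginPlay caches the TimeDecider game instance, and the KickMeoff event starts a self-calling MoveMe loop.
; MoveMe steps the actor forward without sweep on a short delay, or polls more slowly while TimeStopped is set.
; KickMeoff's bounce and color inputs are unused.
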(event Custom|Kick%20Me%20off
  (params (Bounce%20or%20not? :type Boolean) (What%20color%20am%20I? :type Integer))
  (CallFunction|MoveMe))

(event Custom|Move%20Me
  (if (Variables|/Game/Blueprints/TimeDecider.TimeDecider_C|GetTimeStopped (Variables|Default|GetTime%20Decider%20Ref))
    (Utilities|FlowControl|Delay 0.1)
    (CallFunction|MoveMe)
    (else
      (Transformation|SetActorLocation (+ (Transformation|GetActorLocation) (Math|Vector|RotateVector "20.000000, 0, 0" (Transformation|GetActorRotation))) false false)
      (Utilities|FlowControl|Delay 0.01)
      (CallFunction|MoveMe))))

(event EventBeginPlay
  (bind _astime_decider (Utilities|Casting|CastToTimeDecider (Game|GetGameInstance)))
  (Variables|Default|SetTime%20Decider%20Ref _astime_decider))

(fn ConstructionScript
  (|CallParentFunction))