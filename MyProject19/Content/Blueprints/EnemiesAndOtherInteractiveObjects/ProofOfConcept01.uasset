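; Prototype enemy that alternates between chained dashes at the player and short projectile volleys, using a FlipFlop.
; Each dash aims by yaw after a wind-up and damages the player on hit; volleys mix straight shots with randomly angled bouncing ones.
; A shared TimeDelayForAction macro times every action, pauses during time stop, and steps swept dash movement, ending it early when a hit or line trace detects an obstacle.
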(event Custom|Dash%20Forwards
  ;[1 1 1] Dash Action
  (if (Variables|Default|GetDashing)
    (Variables|Default|SetDashes%20Available (- (Variables|Default|GetDashes%20Available) 1.0))
    (Components|Animation|PlayAnimation (Variables|Character|GetMesh) "/Game/Mannequin/Animations/ThirdPersonIdle.ThirdPersonIdle" true)
    (Utilities|TimeDelayforAction 2.5 0.01
      (:NewParam2
        (Variables|Default|SetDashing false)
        (if (== (Variables|Default|GetDashes%20Available) 0.0)
          (Variables|Default|SetDashes%20Available 3.0)
          (CallFunction|DecideNextAction)
          (else
            (CallFunction|DashForwards)))))
    (else
      (Components|Animation|PlayAnimation (Variables|Character|GetMesh) "/Game/Mannequin/Animations/ThirdPersonJump_Loop.ThirdPersonJump_Loop" true)
      (bind _output_get (Variables|Default|SetDash%20Angle (Math|Rotator|MakeRotator 0.0 0.0 (.Yaw (Math|Rotator|BreakRotator (Math|Rotator|FindLookatRotation (Transformation|GetActorLocation) (Transformation|GetActorLocation (Game|Player|GetPlayerPawn 0))))))))
      (Transformation|SetActorRotation _output_get)
      (Utilities|TimeDelayforAction 0.5 0.1
        (:NewParam2
          (Variables|Default|SetDashing true)
          (CallFunction|DashForwards))))))

(event Custom|Decide%20Next%20Action
  (Utilities|FlowControl|FlipFlop
    (:A
      (CallFunction|DashForwards))
    (:B
      (CallFunction|FireProjectiles))))

(event Custom|Fire%20Projectiles
  (bind _returnvalue (Transformation|GetActorTransform))
  (bind (_location _rotation _scale) (Math|Transform|BreakTransform _returnvalue))
  (if (== (Variables|Default|GetProjectiles%20Fired) 0.0)
    (Utilities|TimeDelayforAction 0.5 0.1
      (:NewParam2
        (Variables|Default|SetProjectiles%20Fired 2.0)
        (CallFunction|DecideNextAction)))
    (else
      (Transformation|SetActorRotation (Math|Rotator|MakeRotator 0.0 0.0 (.Yaw (Math|Rotator|BreakRotator (Math|Rotator|FindLookatRotation (Transformation|GetActorLocation) (Transformation|GetActorLocation (Game|Player|GetPlayerPawn 0)))))))
      (if (== (Variables|Default|GetProjectiles%20Fired) 1.0)
        (Utilities|TimeDelayforAction 0.3 0.1
          (:NewParam2
            (bind _returnvalue_2 (Game|SpawnActorfromClass "/Game/Blueprints/EnemiesAndOtherInteractiveObjects/ProofOfConcept01_Projectile.ProofOfConcept01_Projectile_C" (Math|Transform|MakeTransform _location (Math|Rotator|MakeRotator 0.0 0.0 (+ (.Yaw (Math|Rotator|BreakRotator _rotation)) (Math|Random|RandomFloatinRange -5e+01 5e+01))) _scale) "Undefined" 0 0))
            (Default|KickMeOff _returnvalue_2 true)))
        (else
          (Utilities|TimeDelayforAction 0.25 0.1
            (:NewParam2
              (bind _returnvalue_3 (Game|SpawnActorfromClass "/Game/Blueprints/EnemiesAndOtherInteractiveObjects/ProofOfConcept01_Projectile.ProofOfConcept01_Projectile_C" (Transformation|GetActorTransform) "Undefined" 0 0))
              (Default|KickMeOff _returnvalue_3 false)))))
      (Variables|Default|SetProjectiles%20Fired (- (Variables|Default|GetProjectiles%20Fired) 1.0))
      (CallFunction|FireProjectiles))))

(event EventBeginPlay
  (CallFunction|BeginCasts)
  (CallFunction|DecideNextAction))

(event Collision|EventHit
  (params (MyComp :type Primitive%20Component%20Object%20Reference) (Other :type Actor%20Object%20Reference) (OtherComp :type Primitive%20Component%20Object%20Reference) (bSelfMoved :type Boolean) (HitLocation :type Vector :default "0, 0, 0") (HitNormal :type Vector :default "0, 0, 0") (NormalImpulse :type Vector :default "0, 0, 0") (Hit :type Hit%20Result%20Structure%20%28by%20ref%29))
  (if (not (Variables|Default|GetLaunched))
    (if (Variables|Default|GetDashing)
      (if (== (.HitActor (Collision|BreakHitResult Hit)) (Game|Player|GetPlayerPawn 0))
        (bind _asthird_person_character_2d (Utilities|Casting|CastToThirdPersonCharacter2D (Game|Player|GetPlayerPawn 0)))
        (Default|HurtMe _asthird_person_character_2d 4.0 false self)
        (Variables|Default|SetDashed%20Into%20Surface true)))))

(fn ConstructionScript
  (|CallParentFunction))

(fn DashMovement
  (bind _returnvalue (Transformation|GetActorLocation))
  (Transformation|SetActorLocation (+ _returnvalue (Math|Vector|RotateVector "30.000000,0.000000,0.000000" (Variables|Default|GetDash%20Angle))) true false)
  (bind _returnvalue_2 (Collision|LineTraceByChannel _returnvalue (+ _returnvalue (Math|Vector|RotateVector "40.000000,0.000000,0.000000" (Variables|Default|GetDash%20Angle))) "TraceTypeQuery1" false 0 "None"))
  (if _returnvalue_2
    (Variables|Default|SetDashed%20Into%20Surface true)
    (else
      (Development|PrintString "Ey" true true "(R=0.000000,G=0.660000,B=1.000000,A=1.000000)" 0.1))))