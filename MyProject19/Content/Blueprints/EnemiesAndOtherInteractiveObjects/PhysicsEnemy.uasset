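; Physics enemy character that can be knocked flying by pushes once its poise is broken.
; Push drains poise and restarts a timer, which Tick counts down before refilling poise.
; With poise depleted, Push turns the enemy away from the player, enables capsule physics and applies a forward-upward impulse rotated by the passed-in direction.
; Landing only prints debug text, and a freeze-and-resume velocity sequence sits disconnected.
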(event Custom|Push
  (params (NewParam :type Rotator))
  (bind _capsulecomponent (Variables|Default|GetCapsuleComponent))
  (if (<= (Variables|Default|GetPoise_0_0) 0.0)
    (Transformation|SetActorRotation (Math|Rotator|FindLookatRotation (Transformation|GetActorLocation (Game|Player|GetPlayerPawn 0)) (Transformation|GetActorLocation)))
    (Physics|SetSimulatePhysics _capsulecomponent true)
    (Physics|AddImpulse _capsulecomponent (Math|Vector|RotateVector (Math|Vector|MakeVector 2.5e+04 0.0 2.5e+04) NewParam) "None" false)
    (else
      (Variables|Default|SetPoise_0_0 (- (Variables|Default|GetPoise_0_0) 5.0))
      (Variables|Default|SetPoise%20Reset%20Time_0_0 3.0))))

(event EventOnLanded
  (params (Hit :type Hit%20Result%20Structure%20%28by%20ref%29))
  (Development|PrintString "d"))

(event EventTick
  (params (DeltaSeconds :type Float%20%28single-precision%29))
  (if (<= (Variables|Default|GetPoise%20Reset%20Time_0_0) 0.0)
    (Variables|Default|SetPoise_0_0 5.0)
    (else
      (Variables|Default|SetPoise%20Reset%20Time_0_0 (- (Variables|Default|GetPoise%20Reset%20Time_0_0) (* (Utilities|Time|GetWorldDeltaSeconds) (Math|Float|MakeLiteralFloat 1.0)))))))

(event EventBeginPlay)

(fn ConstructionScript
  (|CallParentFunction))