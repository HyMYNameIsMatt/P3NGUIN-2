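; Map transition volume that swaps streamed levels and moves the player to a named spawn point when any actor overlaps it.
; On overlap it loads the target level visibly without blocking, then moves player pawn 0 to the transform of any SpawnPoint whose display name matches the configured point.
; It then unloads the configured current map.
; A cast to TimeDecider is left unconnected and never runs.
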(event EventActorBeginOverlap
  (params (OtherActor :type Actor%20Object%20Reference))
  (Game|LoadStreamLevel(byName) (Variables|Default|GetMapToTransitionTo) true)
  (bind _outactors (Actor|GetAllActorsOfClass "/Game/Blueprints/WorldActors/SpawnPoint.SpawnPoint_C"))
  (for _array_element _outactors
    (if (Utilities|Enum|Equal(Enum) (Utilities|GetDisplayName _array_element) (Variables|Default|GetWhichPointToLoadTo))
      (Transformation|SetActorTransform (Game|Player|GetPlayerPawn 0) (Transformation|GetActorTransform _array_element))))
  (Game|UnloadStreamLevel(byName) (Variables|Default|GetCurrentMapToUnload)))

(fn ConstructionScript)