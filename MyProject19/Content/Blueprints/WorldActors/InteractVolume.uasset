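; InteractVolume is a world actor that lets the player trigger an interaction by pressing E inside its box.
; It enables input on BeginPlay and, on E, checks that the player pawn overlaps the box and is a ThirdPersonCharacter2D not blocked by ScriptIsPreventing.
; It then stores its own display name as the current volume in the TimeDecider game instance and calls a persistent level dispatcher.
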(event EventBeginPlay
  (Input|EnableInput (Game|GetPlayerController 0)))

(event Input|KeyboardEvents|E
  (params (Key :type Key%20Structure :default "AnyKey"))
  (bind _returnvalue (Game|Player|GetPlayerPawn 0))
  (:Pressed
    (if (Collision|IsOverlappingActor (Variables|Default|GetBox) _returnvalue :!class /Script/Engine.PrimitiveComponent)
      (bind _asthird_person_character_2d (Utilities|Casting|CastToThirdPersonCharacter2D _returnvalue)
        (:then
          (if (not (Variables|/Game/Blueprints/2D/Blueprints/Tests/ThirdPersonCharacter2D.ThirdPersonCharacter2D_C|GetScriptIsPreventing _asthird_person_character_2d))
            (bind _astime_decider (Utilities|Casting|CastToTimeDecider (Game|GetGameInstance)))
            (Variables|/Game/Blueprints/TimeDecider.TimeDecider_C|SetCurrentInteractVolume _astime_decider (Utilities|GetDisplayName self))
            (Default|CallPersistantLevelDispatcher)))
        (:CastFailed
          (Development|PrintString "fak"))))))

(fn ConstructionScript)