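; A temporary platform that appears with collision when activated and vanishes after a short countdown.
; It starts hidden, and ActivatePlatform shows the Cube, enables the Box collision and resets the timer.
; Tick counts down only while the TimeDecider game instance reports time is not stopped, so stopping time keeps an active platform in place.
; Once expired, Tick reapplies the BeginPlay hide logic every unpaused frame.
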(event Custom|Activate%20Platform
  (Rendering|SetVisibility (Variables|Default|GetCube) true false)
  (Collision|SetCollisionEnabled (Variables|Default|GetBox) "QueryAndPhysics")
  (Variables|Default|SetTime%20Remaining 0.5))

(event EventBeginPlay
  (bind _astime_decider (Utilities|Casting|CastToTimeDecider (Game|GetGameInstance)))
  (Rendering|SetVisibility (Variables|Default|GetCube) false false)
  (Collision|SetCollisionEnabled (Variables|Default|GetBox) "NoCollision"))

(event EventTick
  (params (DeltaSeconds :type Float%20%28single-precision%29))
  (if (not (Variables|/Game/Blueprints/TimeDecider.TimeDecider_C|GetTimeStopped (stale EventBeginPlay _astime_decider)))
    (if (> (Variables|Default|GetTime%20Remaining) 0.0)
      (Variables|Default|SetTime%20Remaining (- (Variables|Default|GetTime%20Remaining) (* (Utilities|Time|GetWorldDeltaSeconds) (Math|Float|MakeLiteralFloat 1.0))))
      (else
        (Rendering|SetVisibility (Variables|Default|GetCube) false false)
        (Collision|SetCollisionEnabled (Variables|Default|GetBox) "NoCollision")))))

(fn ConstructionScript)