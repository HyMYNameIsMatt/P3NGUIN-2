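; Knife2 is a projectile stand-in that can be held motionless, then replaces itself with a targeted Knife actor.
; BeginKniveing spawns the Knife rotated toward the stored target and destroys this actor.
; Tick freezes it during TimeDecider's time stop, then swaps it for a Knife with the same transform when time resumes, if permitted.
; Overlaps attempt parryable player damage (casting the controller as the character) or damage EnemyBasic actors.
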(event Custom|Begin%20Kniveing
  (Variables|Default|SetCan%20I%20go%20yet? true)
  (bind _returnvalue (Game|SpawnActorfromClass "/Game/Blueprints/Attack_Actors/Knife.Knife_C" (Math|Transform|MakeTransform (.Location (Math|Transform|BreakTransform (Transformation|GetActorTransform))) (Math|Rotator|FindLookatRotation (Transformation|GetActorLocation) (Transformation|GetActorLocation (Variables|Default|GetWho%20I%20Target)))) "Undefined" 0 0))
  (bind _asknife (Utilities|Casting|CastToKnife _returnvalue))
  (CallFunction|SetTarget _asknife (Variables|Default|GetWho%20I%20Target))
  (Actor|DestroyActor))

(event Custom|Establish%20Target
  (params (NewParam :type Actor%20Object%20Reference))
  (Variables|/Script/Engine.ProjectileMovementComponent|SetMaxSpeed (Variables|Default|GetProjectileMovement) 1e-30)
  (Variables|Default|SetWho%20I%20Target NewParam)
  (Variables|Default|SetCan%20I%20go%20yet? false))

(event Custom|Set%20Target
  (params (NewParam :type Actor%20Object%20Reference))
  (Variables|Default|SetWho%20I%20Target NewParam))

(event Custom|Knife%20to%20Meat%20you
  (if (Variables|Default|GetCan%20I%20go%20yet?)
    (bind _returnvalue (Game|SpawnActorfromClass "/Game/Blueprints/Attack_Actors/Knife.Knife_C" (Transformation|GetActorTransform) "Undefined" 0 0))
    (bind _asknife (Utilities|Casting|CastToKnife _returnvalue))
    (CallFunction|SetTarget _asknife (Variables|Default|GetWho%20I%20Target))
    (Actor|DestroyActor)))

(event EventTick
  (params (DeltaSeconds :type Float%20%28single-precision%29))
  (bind _astime_decider (Utilities|Casting|CastToTimeDecider (Game|GetGameInstance)))
  (if (Variables|/Game/Blueprints/TimeDecider.TimeDecider_C|GetTimeStopped _astime_decider)
    (Variables|/Script/Engine.ProjectileMovementComponent|SetMaxSpeed (Variables|Default|GetProjectileMovement) 1e-30)
    (Variables|Default|SetCan%20Be%20Destroyed true)
    (elif (Variables|Default|GetCan%20Be%20Destroyed)
      (CallFunction|KnifetoMeatYou))))

(event Collision|EventActorBeginOverlap
  (params (OtherActor :type Actor%20Object%20Reference))
  (if (== OtherActor (Game|Player|GetPlayerPawn 0))
    (bind _asthird_person_character_2d (Utilities|Casting|CastToThirdPersonCharacter2D (Game|GetPlayerController 0)))
    (Default|HurtMe _asthird_person_character_2d 3.0 true self)
    (Actor|DestroyActor :!label _label)
    (elif (not (== OtherActor "/Game/Blueprints/Attack_Actors/Knife.Knife_C"))
      (bind _asenemy_basic (Utilities|Casting|CastToEnemyBasic OtherActor))
      (Game|Damage|ApplyDamage _asenemy_basic 3.0 0 0)
      (goto _label))))

(fn ConstructionScript)