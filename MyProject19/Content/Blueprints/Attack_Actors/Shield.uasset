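; Short-lived shield actor that parries enemy attacks and rewards the player for it.
; Once shielding begins, it destroys itself after a half-second delay.
; Any overlapping EnemyAttacks actor is destroyed; the shield then casts to the player's ThirdPersonCharacter2D and plays a parry sound.
; Each parry adds to the player's time bar, or to magic if that bar is full, and calls the matching update function.
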(event Custom|Begin%20Shielding
  (Utilities|FlowControl|Delay 0.5)
  (Actor|DestroyActor))

(event Collision|EventActorBeginOverlap
  (params (OtherActor :type Actor%20Object%20Reference))
  (if (Utilities|ClassIsChildOf (Utilities|GetClass OtherActor) "/Game/Blueprints/EnemyAttacks.EnemyAttacks_C")
    (Actor|DestroyActor OtherActor)
    (bind _asthird_person_character_2d (Utilities|Casting|CastToThirdPersonCharacter2D (Game|Player|GetPlayerPawn 0)))
    (Variables|Default|SetPlayer%20Stats _asthird_person_character_2d)
    (Audio|PlaySound2D "/Game/Blueprints/SoundEffects/parryyes.parryyes")
    (if (>= (Variables|/Game/Blueprints/2D/Blueprints/Tests/ThirdPersonCharacter2D.ThirdPersonCharacter2D_C|GetTimeBar (Variables|Default|GetPlayer%20Stats)) (Variables|/Game/Blueprints/2D/Blueprints/Tests/ThirdPersonCharacter2D.ThirdPersonCharacter2D_C|GetTimeBarMax (Variables|Default|GetPlayer%20Stats)))
      (Variables|/Game/Blueprints/2D/Blueprints/Tests/ThirdPersonCharacter2D.ThirdPersonCharacter2D_C|SetCurrentMagic (Variables|Default|GetPlayer%20Stats) (+ 2.0 (Variables|/Game/Blueprints/2D/Blueprints/Tests/ThirdPersonCharacter2D.ThirdPersonCharacter2D_C|GetCurrentMagic (Variables|Default|GetPlayer%20Stats))))
      (Default|UpdateMagic (Variables|Default|GetPlayer%20Stats))
      (else
        (Variables|/Game/Blueprints/2D/Blueprints/Tests/ThirdPersonCharacter2D.ThirdPersonCharacter2D_C|SetTimeBar (Variables|Default|GetPlayer%20Stats) (+ (Variables|/Game/Blueprints/2D/Blueprints/Tests/ThirdPersonCharacter2D.ThirdPersonCharacter2D_C|GetTimeBar (Variables|Default|GetPlayer%20Stats)) 2.0))
        (Default|UpdateTime (Variables|Default|GetPlayer%20Stats))))))

(fn ConstructionScript)