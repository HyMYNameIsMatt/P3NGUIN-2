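; Healer is an attack actor that restores a fixed amount of the player's health when its BeginHealing event runs.
; It plays a status sound, casts the player pawn to ThirdPersonCharacter2D and raises Health, capped at MaxHealth.
; It then calls the character's TakeDamage with zero damage and destroys itself, after a short delay if the cap was not reached.
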(event Custom|Begin%20Healing
  (Audio|PlaySound2D "/Game/Blueprints/SoundEffects/Damage/StatusPositive.StatusPositive")
  (bind _asthird_person_character_2d (Utilities|Casting|CastToThirdPersonCharacter2D (Game|Player|GetPlayerPawn 0)))
  (bind _output_get (Variables|Default|SetPlayer%20Stats _asthird_person_character_2d))
  (if (>= (+ (Variables|/Game/Blueprints/2D/Blueprints/Tests/ThirdPersonCharacter2D.ThirdPersonCharacter2D_C|GetHealth _output_get) 5.0) (Variables|/Game/Blueprints/2D/Blueprints/Tests/ThirdPersonCharacter2D.ThirdPersonCharacter2D_C|GetMaxHealth _output_get))
    (Variables|/Game/Blueprints/2D/Blueprints/Tests/ThirdPersonCharacter2D.ThirdPersonCharacter2D_C|SetHealth _output_get (Variables|/Game/Blueprints/2D/Blueprints/Tests/ThirdPersonCharacter2D.ThirdPersonCharacter2D_C|GetMaxHealth _output_get))
    (else
      (Variables|/Game/Blueprints/2D/Blueprints/Tests/ThirdPersonCharacter2D.ThirdPersonCharacter2D_C|SetHealth _output_get (+ (Variables|/Game/Blueprints/2D/Blueprints/Tests/ThirdPersonCharacter2D.ThirdPersonCharacter2D_C|GetHealth _output_get) 5.0))
      (Utilities|FlowControl|Delay 0.1)))
  (Default|TakeDamage (Variables|Default|GetPlayer%20Stats) 0 0.0)
  (Actor|DestroyActor))

(fn ConstructionScript)