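; Knife attack actor that hits a stored target with an instant line trace, then destroys itself.
; EstablishTarget stores the target, and BeginKniveing traces to it on the Visibility channel with debug drawing.
; Whatever the trace hits takes fixed damage and a particle spawns with the impact point as its location.
; GiveTimeBackKnife is a stub that only casts the player controller to ThirdPersonCharacter2D.
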(event Custom|Begin%20Kniveing
  (bind _outhit (Collision|LineTraceByChannel (Transformation|GetActorLocation) (Transformation|GetActorLocation (Variables|Default|GetWho%20I%20Target)) "TraceTypeQuery1" false 0 "ForDuration"))
  (Game|Damage|ApplyDamage (.HitActor (Collision|BreakHitResult _outhit)) 3.0 0 0)
  (Effects|SpawnEmitterAttached "/Game/Defaultpparticle.Defaultpparticle" 0 "None" (.ImpactPoint (Collision|BreakHitResult _outhit)))
  (Actor|DestroyActor))

(event Custom|Establish%20Target
  (params (NewParam :type Actor%20Object%20Reference))
  (Variables|Default|SetWho%20I%20Target NewParam))

(event Custom|Give%20Time%20Back%20Knife
  (Utilities|Casting|CastToThirdPersonCharacter2D (Game|GetPlayerController 0)))

(fn ConstructionScript)