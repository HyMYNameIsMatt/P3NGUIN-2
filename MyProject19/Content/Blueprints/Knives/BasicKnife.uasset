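; BasicKnife is a homing knife projectile that damages actors it overlaps, ignoring the player and other knives, then destroys itself.
; Each tick it scans EnemyBasic actors within a yaw cone and range to set its homing target, though any failing candidate clears the current pick.
; When the TimeDecider game instance stops time, it halts movement, then replaces itself with a fresh copy at the same transform once time resumes.
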(event Collision|EventActorBeginOverlap
  (params (OtherActor :type Actor%20Object%20Reference))
  (if (not (== OtherActor (Game|Player|GetPlayerPawn 0)))
    (if (not (Utilities|ClassIsChildOf (Utilities|GetClass OtherActor) "/Game/Blueprints/Knives/KnifeParent.KnifeParent_C"))
      (Game|Damage|ApplyDamage OtherActor 5.0 0 0)
      (Actor|DestroyActor))))

(event EventBeginPlay
  (bind _projectilemovement (Variables|Default|GetProjectileMovement))
  (Variables|Default|SetClosest%20Distance (Variables|Default|GetMinimum%20Distance%20EDIT))
  (bind _output_get (Variables|/Script/Engine.ProjectileMovementComponent|SetMaxSpeed _projectilemovement (Variables|Default|GetKnife%20Speed%20EDIT)))
  (Variables|/Script/Engine.ProjectileMovementComponent|SetInitialSpeed _projectilemovement _output_get)
  (Variables|/Script/Engine.ProjectileMovementComponent|SetHomingAccelerationMagnitude _projectilemovement (Variables|Default|GetHoming%20Rate%20EDIT)))

(event EventTick
  (params (DeltaSeconds :type Float%20%28single-precision%29))
  (bind _projectilemovement (Variables|Default|GetProjectileMovement))
  (bind _projectilemovement_2 (Variables|Default|GetProjectileMovement))
  (bind _minimumangle_edit (Variables|Default|GetMinimumAngle%20EDIT))
  (bind _astime_decider (Utilities|Casting|CastToTimeDecider (Game|GetGameInstance)))
  (if (Variables|/Game/Blueprints/TimeDecider.TimeDecider_C|GetTimeStopped _astime_decider)
    (Variables|Default|SetNeeds%20to%20respawn true)
    (Variables|Default|SetClosest%20Distance 0.0)
    (bind _output_get (Variables|/Script/Engine.ProjectileMovementComponent|SetMaxSpeed _projectilemovement_2 0.0))
    (Variables|/Script/Engine.ProjectileMovementComponent|SetInitialSpeed _projectilemovement_2 _output_get)
    (Variables|/Script/Engine.ProjectileMovementComponent|SetHomingAccelerationMagnitude _projectilemovement_2 0.0)
    (Game|Components|ProjectileMovement|StopSimulating (Variables|Default|GetProjectileMovement) (Collision|MakeHitResult))
    (elif (Variables|Default|GetNeeds%20to%20respawn)
      (Game|SpawnActorfromClass "BasicKnife_C" (Transformation|GetActorTransform) "Undefined" 0 0)
      (Actor|DestroyActor)
      (else
        (bind _outactors (Actor|GetAllActorsOfClass "/Game/Blueprints/EnemiesAndOtherInteractiveObjects/EnemyBasic.EnemyBasic_C"))
        (for _array_element _outactors
          (if (and (< (- (.Yaw (Math|Rotator|BreakRotator (Transformation|GetActorRotation))) (.Yaw (Math|Rotator|BreakRotator (Math|Rotator|FindLookatRotation (Transformation|GetActorLocation) (Transformation|GetActorLocation _array_element))))) _minimumangle_edit) (> (- (.Yaw (Math|Rotator|BreakRotator (Transformation|GetActorRotation))) (.Yaw (Math|Rotator|BreakRotator (Math|Rotator|FindLookatRotation (Transformation|GetActorLocation) (Transformation|GetActorLocation _array_element))))) (* -1 _minimumangle_edit)))
            (if (and (> (Transformation|GetDistanceTo _array_element self) 1.0) (< (Transformation|GetDistanceTo _array_element self) (Variables|Default|GetClosest%20Distance)))
              (Variables|Default|SetNearest _array_element)
              (Variables|Default|SetClosest%20Distance (Transformation|GetDistanceTo _array_element self))
              (else
                (Variables|Default|SetNearest 0 :!label _label)))
            (else
              (goto _label))))
        (Variables|Default|SetClosest%20Distance (Variables|Default|GetMinimum%20Distance%20EDIT))
        (bind _asenemy_basic (Utilities|Casting|CastToEnemyBasic (Variables|Default|GetNearest))
          (:then
            (Variables|/Script/Engine.ProjectileMovementComponent|SetHomingTargetComponent _projectilemovement (Variables|/Script/Engine.Character|GetCapsuleComponent _asenemy_basic)))
          (:CastFailed
            (Variables|/Script/Engine.ProjectileMovementComponent|SetHomingTargetComponent _projectilemovement 0)
            (Development|PrintString "Hello" true true "(R=0.000000,G=1.000000,B=0.549564,A=1.000000)" 0.1)))))))

(fn ConstructionScript
  (|CallParentFunction))