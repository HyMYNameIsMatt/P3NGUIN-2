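; Generic enemy character that faces the player and attacks with bullets and poison shots, pausing its AI while the game instance's TimeStopped is set.
; Tick lunges forward when off-screen, otherwise randomly picks a three-way spread, poison shot or side dodge, sometimes leaping back at close range.
; A BusyRightNow flag with a delay spaces most actions.
; Damage lowers Health and updates a floating health bar, with no death handling here.
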(event Custom|Spread%20Shot
  (bind _returnvalue (Transformation|GetActorRotation))
  (bind _returnvalue_2 (Transformation|GetActorRotation))
  (bind _self self)
  (bind (_roll _pitch _yaw) (Math|Rotator|BreakRotator _returnvalue))
  (bind (_roll_2 _pitch_2 _yaw_2) (Math|Rotator|BreakRotator _returnvalue_2))
  ;[1 1 1] SpreadShot
  (Game|SpawnActorfromClass "/Game/Blueprints/IAMBULLETHELLO.IAMBULLETHELLO_C" (Math|Transform|MakeTransform (Transformation|GetActorLocation) (Transformation|GetActorRotation)) "Undefined" 0 _self)
  (Game|SpawnActorfromClass "/Game/Blueprints/IAMBULLETHELLO.IAMBULLETHELLO_C" (Math|Transform|MakeTransform (Transformation|GetActorLocation) (Math|Rotator|MakeRotator _roll_2 _pitch_2 (+ _yaw_2 3e+01))) "Undefined" 0 _self)
  (Game|SpawnActorfromClass "/Game/Blueprints/IAMBULLETHELLO.IAMBULLETHELLO_C" (Math|Transform|MakeTransform (Transformation|GetActorLocation) (Math|Rotator|MakeRotator _roll _pitch (+ _yaw -3e+01))) "Undefined" 0 _self)
  (Variables|Default|SetBusyRightNow true))

(event Custom|PoisonShot
  ;[1 1 1] Poison Shot
  (Game|SpawnActorfromClass "/Game/Blueprints/Poison.Poison_C" (Math|Transform|MakeTransform (Transformation|GetActorLocation) (Transformation|GetActorRotation)) "Undefined" 0 self)
  (Variables|Default|SetBusyRightNow true))

(event Custom|Dodge
  (bind _returnvalue (Transformation|GetActorRotation))
  (bind _returnvalue_2 (Math|Vector|GetRightVector _returnvalue))
  ;[1 1 1] Dodgetoleftorright
  (if (Math|Random|RandomBool)
    (Character|LaunchCharacter (* _returnvalue_2 2500) false false)
    (else
      (Character|LaunchCharacter (* _returnvalue_2 -2500) false false))))

(event Custom|MoveForward
  ;[1 1 1] DodgeForward
  (Character|LaunchCharacter (* (Math|Vector|GetForwardVector (Transformation|GetActorRotation)) 5000) false false)
  (Variables|Default|SetBusyRightNow true))

(event Custom|Dodge%20Back
  ;[1 1 1] MoveBack
  (Character|LaunchCharacter (* (Math|Vector|GetForwardVector (Transformation|GetActorRotation)) -2500) false false)
  (Variables|Default|SetBusyRightNow true))

(event Game|Damage|EventAnyDamage
  (params (Damage :type Float%20%28single-precision%29) (DamageType :type Damage%20Type%20Object%20Reference) (InstigatedBy :type Controller%20Object%20Reference) (DamageCauser :type Actor%20Object%20Reference))
  ;[1 1 1] TakeDamage
  (bind _output_get (Variables|Default|SetHealth (- (Variables|Default|GetHealth) Damage)))
  (CallFunction|SendHealthtoBar _output_get)
  (Development|PrintString (Utilities|String|ToString(Float) _output_get) true true "(R=1.000000,G=0.061744,B=0.000000,A=1.000000)"))

(event EventBeginPlay
  (bind _asenemy_health (Utilities|Casting|CastToEnemyHealth (UserInterface|GetUserWidgetObject (Variables|Default|GetHP))))
  (Variables|Default|SetEnemyHealth _asenemy_health)
  (Variables|Default|SetHealth 5e+01)
  (Variables|Default|SetMaxHealth 5e+01))

(event EventTick
  (params (DeltaSeconds :type Float%20%28single-precision%29))
  (bind _returnvalue (Game|GetPlayerController 0))
  (bind _returnvalue_2 (Transformation|GetActorLocation))
  (bind _returnvalue_3 (Viewport|GetViewportSize))
  (bind _returnvalue_4 (Math|Random|RandomIntegerinRange 0 8))
  (bind _screenlocation (Class|PlayerController|ProjectWorldLocationtoScreen _returnvalue _returnvalue_2))
  (bind (_x _y) (Math|Vector2D|BreakVector2D _returnvalue_3))
  (bind (_x_2 _y_2) (Math|Vector2D|BreakVector2D _screenlocation))
  (Transformation|SetRelativeLocation (Variables|Default|GetHP) (+ (Transformation|GetActorLocation) "0,0.000000,100.000000") false false)
  ;[1 1 1] PickAction
  (bind _astime_decider (Utilities|Casting|CastToTimeDecider (Game|GetGameInstance)))
  (if (not (Variables|/Game/Blueprints/TimeDecider.TimeDecider_C|GetTimeStopped _astime_decider))
    (Transformation|SetActorRelativeRotation (Math|Rotator|FindLookatRotation (Transformation|GetActorLocation self) (Transformation|GetActorLocation (Game|Player|GetPlayerPawn 0))))
    (if true
      (if (Variables|Default|GetBusyRightNow)
        (Utilities|FlowControl|Delay 2.5)
        (Variables|Default|SetBusyRightNow false)
        (elif (Math|Boolean|ANDBoolean (> _x_2 0.0) (> _y_2 0.0) (< _x_2 _x) (< _y_2 _y))
          (if (<= 3e+02 (Transformation|GetDistanceTo (Game|Player|GetPlayerPawn 0)))
            (if (== _returnvalue_4 8) :!label _label
              (CallFunction|PoisonShot)
              (elif (== _returnvalue_4 7)
                (CallFunction|Dodge)
                (else
                  (CallFunction|SpreadShot))))
            (elif (Math|Random|RandomBool)
              (goto _label)
              (else
                (CallFunction|DodgeBack))))
          (else
            (CallFunction|MoveForward)))))))

(fn ConstructionScript
  (|CallParentFunction))