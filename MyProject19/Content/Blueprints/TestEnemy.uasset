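; Test enemy that chases the player when nearby and otherwise returns to its spawn location.
; Tick halts movement while the TimeDecider game instance has time stopped, and handles death with a particle burst and cleanup.
; Taking damage lowers health, updates the bar and deals fixed damage back to the player.
; Its viewport health widget follows the capsule through world-to-screen projection with a hardcoded offset.
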(event Game|Damage|EventAnyDamage
  (params (Damage :type Float%20%28single-precision%29) (DamageType :type Damage%20Type%20Object%20Reference) (InstigatedBy :type Controller%20Object%20Reference) (DamageCauser :type Actor%20Object%20Reference))
  (Game|Damage|ApplyDamage (Game|GetPlayerCharacter 0) 8.0 0 self "/Script/Engine.DamageType")
  (bind _output_get (Variables|Default|SetHealth (- (Variables|Default|GetHealth) Damage)))
  (CallFunction|SendHealthtoBar _output_get)
  (Development|PrintString (Utilities|String|ToString(Float) _output_get) true true "(R=1.000000,G=0.061744,B=0.000000,A=1.000000)"))

(event EventBeginPlay
  (bind _returnvalue (UserInterface|CreateWidget "/Game/Blueprints/UI/EnemyHealth.EnemyHealth_C"))
  (bind _output_get (Variables|Default|SetEnemyHealth _returnvalue))
  (UserInterface|Viewport|AddtoViewport _output_get 0)
  (Variables|Default|SetStartingLocation (Transformation|GetActorLocation))
  (CallFunction|SendHealthtoBar (Variables|Default|GetHealth)))

(event EventTick
  (params (DeltaSeconds :type Float%20%28single-precision%29))
  (bind _returnvalue (Pawn|GetController))
  (Utilities|FlowControl|Sequence
    (:then_0
      (bind _astime_decider (Utilities|Casting|CastToTimeDecider (Game|GetGameInstance)))
      (if (Variables|/Game/Blueprints/TimeDecider.TimeDecider_C|GetTimeStopped _astime_decider)
        (AI|Navigation|StopMovement (Pawn|GetController))
        (else
          (Utilities|FlowControl|Sequence
            (:then_1
              (if (Math|Vector|Equal(Vector) (Transformation|GetActorLocation (Game|Player|GetPlayerPawn 0)) (Transformation|GetActorLocation) 5e+02)
                (AI|Navigation|SimpleMovetoActor _returnvalue (Game|Player|GetPlayerPawn 0))
                (else
                  (AI|Navigation|SimpleMovetoLocation _returnvalue (Variables|Default|GetStartingLocation)))))))))
    (:then_1
      (if (<= (Variables|Default|GetHealth) 0.0)
        (Effects|SpawnEmitteratLocation "/Game/Defaultpparticle.Defaultpparticle" (Transformation|GetActorLocation))
        (Widget|RemovefromParent (Variables|Default|GetEnemyHealth))
        (Actor|DestroyActor)))
    (:then_2
      (CallFunction|SetHealthBarLocation))))

(fn ConstructionScript)

(fn SendHealthtoBar
  (params (Enemy%20Health :type Float%20%28single-precision%29))
  (Variables|/Game/Blueprints/UI/EnemyHealth.EnemyHealth_C|SetHealthPercentageEnemy (Variables|Default|GetEnemyHealth) (/ Enemy%20Health (Variables|Default|GetMaxHealth))))

(fn SetHealthBarLocation
  (bind _asenemy_health (Utilities|Casting|CastToEnemyHealth (Variables|Default|GetEnemyHealth)))
  (Default|SetLocation _asenemy_health (+ (.ScreenLocation (Class|PlayerController|ProjectWorldLocationtoScreen (Game|GetPlayerController 0) (Transformation|GetWorldLocation (Variables|Collision|GetCapsuleComponent)))) "(X=-645.000000,Y=-450.000000)")))