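; Poison projectile that hurts the ThirdPersonCharacter2D on overlap with a parryable, special-condition hit, then destroys itself.
; Each tick it reads TimeStopped from the TimeDecider game instance and, while time is stopped, zeroes its projectile max speed and flags itself.
; When time resumes, a flagged projectile spawns a fresh copy at its cylinder's location and rotation, then destroys itself rather than restoring speed.
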(event EventTick
  (params (DeltaSeconds :type Float%20%28single-precision%29))
  (Utilities|FlowControl|Sequence
    (:then_0
      (bind _astime_decider (Utilities|Casting|CastToTimeDecider (Game|GetGameInstance)))
      (if (Variables|/Game/Blueprints/TimeDecider.TimeDecider_C|GetTimeStopped _astime_decider)
        (Variables|/Script/Engine.ProjectileMovementComponent|SetMaxSpeed (Variables|Default|GetProjectileMovement) 1e-12)
        (Variables|Default|SetCanBeDestroyed true)
        (elif (Variables|Default|GetCanBeDestroyed)
          (Game|SpawnActorfromClass "Poison_C" (Math|Transform|MakeTransform (Transformation|GetWorldLocation (Variables|Default|GetCylinder)) (Transformation|GetActorRotation)) "Undefined" 0 0)
          (Actor|DestroyActor))))))

(event Collision|EventActorBeginOverlap
  (params (OtherActor :type Actor%20Object%20Reference))
  (if (== (Utilities|GetClass OtherActor) "/Game/Blueprints/2D/Blueprints/Tests/ThirdPersonCharacter2D.ThirdPersonCharacter2D_C")
    (bind _asthird_person_character_2d (Utilities|Casting|CastToThirdPersonCharacter2D OtherActor))
    (Default|HurtMe _asthird_person_character_2d 2.0 true self 1)
    (Actor|DestroyActor)))

(fn ConstructionScript)